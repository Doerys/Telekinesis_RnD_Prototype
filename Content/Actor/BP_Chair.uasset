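; Physics chair prop that the player can levitate, pull toward themselves and launch.
; OnInteract toggles levitation, switching mesh gravity and playing a timeline that drives the mesh's relative Z when lifting.
; Attract moves the mesh to the player pawn's location with MoveComponentTo, zeroing velocity on completion, and Stop halts that move.
; Propulse applies a velocity-change impulse, restores gravity and clears the levitation flag.
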(event EventPropulse
  (params (PropulseLocation :type Vector :default "0, 0, 0"))
  (Physics|AddImpulse (Variables|Default|GetSM_Chair) PropulseLocation "None" true)
  (Physics|SetEnableGravity (Variables|Default|GetSM_Chair) true)
  (Variables|Default|SetIsLevitating_0 false))

(event EventAttract
  (params (IsComing :type Character%20Object%20Reference))
  (Components|MoveComponentTo (Variables|Default|GetSM_Chair) (Transformation|GetActorLocation (Game|Player|GetPlayerPawn 0)) "0, 0, 0" false false 1.0 false)
  (Physics|SetPhysicsLinearVelocity (Variables|Default|GetSM_Chair) "0, 0, 0" false "None"))

(event EventStop
  (params (InteractingPlayer :type Character%20Object%20Reference))
  (Components|MoveComponentTo (Variables|Default|GetSM_Chair) (Transformation|GetActorLocation (Game|Player|GetPlayerPawn 0)) "0, 0, 0" false false 1.0 false) ; enters at Stop
)

(event EventOnInteract
  (params (InteractingPlayer :type Character%20Object%20Reference))
  (bind _sm_chair (Variables|Default|GetSM_Chair))
  (bind _relativelocation (Variables|/Script/Engine.SceneComponent|GetRelativeLocation _sm_chair))
  (if (Variables|Default|GetIsLevitating_0)
    (Development|PrintString "oulala je vole plus")
    (Variables|Default|SetIsLevitating_0 false)
    (CallFunction|Levitate?)
    (Physics|SetEnableGravity (Variables|Default|GetSM_Chair) true)
    (else
      (Development|PrintString "oulala je vole")
      (Variables|Default|SetIsLevitating_0 true)
      (CallFunction|Levitate?)
      (Physics|SetEnableGravity (Variables|Default|GetSM_Chair) false)
      (bind _float (Timeline|StartLevitate PlayFromStart)
        (:Update
          (Transformation|SetRelativeLocation (Variables|Default|GetSM_Chair) (Math|Vector|MakeVector (.x _relativelocation) (.y _relativelocation) _float) false false))))))

(fn ConstructionScript)

(fn IsInteractable
  (return false))

(fn Levitate?
  (if (Variables|Default|GetIsLevitating_0)
    (return true)
    (else
      (return false))))