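; BP_SMFinder is a helper actor that finds and stores a static mesh component on its attach parent actor.
; On BeginPlay it caches that component in UsableMesh and prints its name for debugging.
; An unconnected chain would disable gravity on the mesh and animate its relative Z with a timeline.
; IsInteractable and Levitate both return false, so levitation is inactive.
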(event EventBeginPlay
  (bind _returnvalue (Actor|GetAttachParentActor))
  (bind _returnvalue_2 (Actor|GetComponentbyClass _returnvalue "/Script/Engine.StaticMeshComponent"))
  (Development|PrintString (Utilities|GetDisplayName _returnvalue_2))
  (bind _output_get (Variables|Default|SetUsable%20Mesh _returnvalue_2))
  (Development|PrintString (Utilities|GetDisplayName _output_get)))

(fn ConstructionScript)

(fn IsInteractable
  (return false))

(fn Levitate?
  (return false))