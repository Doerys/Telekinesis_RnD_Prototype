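; Prototype telekinesis interactive prop that can be grabbed, carried and thrown.
; OnGrab pulls light objects to a target with gravity off, and MaintainGrab then sweeps the actor along with supplied location and rotation.
; OnRelease applies a velocity-change impulse and restores gravity after a delay, or on a cube hit while ungrabbed.
; Heavy objects only call Levitate and IsDropped; the behavior hooks are mostly empty stubs.
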(event OnComponentHit(Shape_Cube)
  (params (HitComponent :type Primitive%20Component%20Object%20Reference) (OtherActor :type Actor%20Object%20Reference) (OtherComp :type Primitive%20Component%20Object%20Reference) (NormalImpulse :type Vector :default "0, 0, 0") (Hit :type Hit%20Result%20Structure%20%28by%20ref%29))
  (if (not (Variables|Default|GetisGrabbed))
    (if (not (Class|PrimitiveComponent|IsGravityEnabled (Variables|Default|GetUsable%20Mesh)))
      (Physics|SetEnableGravity (Variables|Default|GetUsable%20Mesh) true))))

(event Custom|Event%20OnGrab
  (params (AttractionSpeed :type Float%20%28double-precision%29) (Target%20Location :type Vector))
  (Variables|Default|SetisGrabbed true)
  (if (Variables|Default|GetisHeavy)
    (CallFunction|Levitate)
    (else
      (CallFunction|IsAttracted)
      (Components|MoveComponentTo (Variables|Default|GetUsable%20Mesh) Target%20Location "0, 0, 0" false false AttractionSpeed false)
      (Variables|Default|SetreachedPlayer true)
      (Physics|SetEnableGravity (Variables|Default|GetUsable%20Mesh) false)
      (Development|PrintString "Reached player"))))

(event Custom|Event%20MaintainGrab
  (params (Target%20Location :type Vector) (PlayerRotation :type Rotator))
  (if (Variables|Default|GetreachedPlayer)
    (Transformation|SetActorRotation PlayerRotation)
    (Transformation|SetActorLocation Target%20Location true false)
    (Development|PrintString "Suis le joueur")))

(event Custom|Event%20OnRelease
  (params (ProjectLocation :type Vector) (ProjectionStrenght :type Float%20%28double-precision%29))
  (if (Variables|Default|GetisHeavy)
    (CallFunction|IsDropped)
    (else
      (CallFunction|IsThrown)
      (Physics|AddImpulse (Variables|Default|GetUsable%20Mesh) (* ProjectLocation ProjectionStrenght) "None" true)
      (Rendering|Material|SetMaterial (Variables|Default|GetUsable%20Mesh) 0 (Variables|Default|GetBaseMaterial))
      (Development|PrintString "Input Release")
      (Variables|Default|SetisGrabbed false)
      (Utilities|FlowControl|Delay 2.0)
      (Physics|SetEnableGravity (Variables|Default|GetUsable%20Mesh) true))))

(event EventBeginPlay
  (CallFunction|Start))

(fn ConstructionScript)

(fn Start
  (bind _returnvalue (Actor|GetComponentbyClass "/Script/Engine.StaticMeshComponent"))
  (Utilities|FlowControl|Sequence
    (:then_0
      (bind _output_get (Variables|Default|SetUsable%20Mesh _returnvalue))
      (Variables|Default|SetBaseMaterial (Rendering|Material|GetMaterial _output_get 0)))
    (:then_1
      (Development|PrintString (Utilities|GetDisplayName _returnvalue)))))

(fn Levitate)

(fn IsDropped)

(fn IsAttracted)

(fn IsThrown)

(fn IsInteractable
  (return false))

(fn Levitate?
  (if true
    (return true)
    (else
      (return false))))